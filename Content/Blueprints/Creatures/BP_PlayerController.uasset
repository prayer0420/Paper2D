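; Player controller that turns movement axis input into state and facing for the controlled BP_Knight.
; It caches the knight on BeginPlay and polls input every Tick while the knight is in Idle or Move.
; It picks Move while the destination is unreached or MoveUp is held; MoveRight is left out of this check.
; Both axes set Direction, with horizontal overriding vertical, and StopMove is set when neither is pressed.
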(event EventBeginPlay
  (bind _asbp_knight (Utilities|Casting|CastToBP_Knight (Pawn|GetControlledPawn)))
  (Variables|Default|SetMyPlayer _asbp_knight))

(event EventTick
  (params (DeltaSeconds :type Float%20%28single-precision%29))
  (CallFunction|UpdateInput))

(fn ConstructionScript)

(fn UpdateInput
  (bind _myplayer (Variables|Default|GetMyPlayer))
  (bind _myplayer_2 (Variables|Default|GetMyPlayer))
  (bind _myplayer_3 (Variables|Default|GetMyPlayer))
  (bind _barrived (Default|HasArrivedtoDest _myplayer_2))
  (bind _returnvalue (not _barrived))
  (switch Utilities|FlowControl|Switch|SwitchonEState (Variables|/Game/Blueprints/Creatures/BP_Creature.BP_Creature_C|GetState (Variables|Default|GetMyPlayer))
    (:NewEnumerator0
      _)
    (:NewEnumerator1
      _))
  (Utilities|FlowControl|Sequence
    (:then_0
      ;[1 1 1] 목적지까지 도착안했거나 , up&right 중 입력을 누르고 있으면 Move, 아니면 Idle
      (if (Math|Boolean|ORBoolean _returnvalue (!= (Input|AxisValues|GetMoveUp) 0.0) _returnvalue)
        (Variables|/Game/Blueprints/Creatures/BP_Creature.BP_Creature_C|SetState _myplayer_3 "NewEnumerator1")
        (else
          (Variables|/Game/Blueprints/Creatures/BP_Creature.BP_Creature_C|SetState _myplayer_3 "NewEnumerator0"))))
    (:then_1
      ;[1 1 1] 이동상태라면(Axis MoveUp) value(1 또는 -1)에 따라 Up, Down
      (Math|Float|CompareFloat (Input|AxisValues|GetMoveUp) 0.0
        (:>
          (Variables|/Game/Blueprints/Creatures/BP_Creature.BP_Creature_C|SetDirection _myplayer "NewEnumerator0"))
        (:<
          (Variables|/Game/Blueprints/Creatures/BP_Creature.BP_Creature_C|SetDirection _myplayer "NewEnumerator1"))))
    (:then_2
      ;[1 1 1] 이동상태라면(Axis MoveRight) value(1 또는 -1)에 따라 Right, Left
      (Math|Float|CompareFloat (Input|AxisValues|GetMoveRight) 0.0
        (:>
          (Variables|/Game/Blueprints/Creatures/BP_Creature.BP_Creature_C|SetDirection _myplayer "NewEnumerator3"))
        (:<
          (Variables|/Game/Blueprints/Creatures/BP_Creature.BP_Creature_C|SetDirection _myplayer "NewEnumerator2"))))
    (:then_3
      ;[1 1 1] 상하좌우 입력을 안했다면 멈춰
      (Variables|/Game/Blueprints/Creatures/BP_Creature.BP_Creature_C|SetbStopMove (Variables|Default|GetMyPlayer) (and (== (Input|AxisValues|GetMoveUp) 0.0) (== (Input|AxisValues|GetMoveRight) 0.0))))))