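; BP_TileMap is a Paper2D tile map actor that serves as a walkability grid for grid-based movement.
; On BeginPlay it sizes a boolean array to the map and flags layer 1 tiles as blocked, assuming a hardcoded width of 10.
; CanGo bounds-checks a cell and reports whether it is unblocked.
; GetTilePos converts cells to world locations on the XZ plane, growing downward from the actor, with a validity flag.
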(event EventBeginPlay
  (bind _rendercomponent (Variables|Default|GetRenderComponent))
  (bind _tilemap (Variables|/Script/Paper2D.PaperTileMapComponent|GetTileMap _rendercomponent))
  (Utilities|FlowControl|Sequence
    (:then_0
      ;[1 1 1] 배열의 크기를 타일맵의 크기랑 같도록 설정(Set MapWidth, MapHeight)
      (Utilities|Array|Resize (Variables|Default|GetMapGrid) (* (Variables|/Script/Paper2D.PaperTileMap|GetMapWidth _tilemap) (Variables|/Script/Paper2D.PaperTileMap|GetMapHeight _tilemap)))
      (Variables|Default|SetMapWidth (Variables|/Script/Paper2D.PaperTileMap|GetMapWidth _tilemap))
      (Variables|Default|SetMapHeight (Variables|/Script/Paper2D.PaperTileMap|GetMapHeight _tilemap)))
    (:then_1
      ;[1 1 1] 배열을 한개씩 순회해서 1번레이어의 타일이 있는지 없는지 확인 해서 타일이 있다면                                                                                           다시 배열의 각 인덱스 값에 true를 넣어줌  벽으로 막혀있는것)
      (for (_ _array_index) (Variables|Default|GetMapGrid)
        (Utilities|IsValid (.tileset (Class|PaperTileMapComponent|GetTile (Variables|Default|GetRenderComponent) (Math|Integer|%(Integer) _array_index 10) (/ _array_index 10) 1))
          (:Is%20Valid
            (Utilities|Array|SetArrayElem (Variables|Default|GetMapGrid) _array_index true)))))))

(fn ConstructionScript)

(fn CanGo
  (params (GirdX :type Integer) (GirdY :type Integer))
  ;[1 1 1] 배열의 2차원좌표를 인덱스로 변환하고, 그 인덱스의 bool값을 뒤집어서 return함.             기본적으로 다 false이고, tile이 있는곳은 막혀있는곳인데 true로 되어있으니까 바꿔줘서 기본적으로 true이고 막혀있는곳만 false가 되도록
  (bind (_bvalid _index) (CallFunction|GridPositiontoIndex GirdX GirdY))
  (if _bvalid
    (return (not (Utilities|Array|Get(acopy) (Variables|Default|GetMapGrid) _index)))
    (else
      (return false))))

(fn GridPositiontoIndex
  (params (GridX :type Integer) (GridY :type Integer))
  ;[1 1 1] TileMap의 X와Y좌표의 범위를 설정하고 인덱스 값으로 바꿔서 Return
  (return (and (Math|Integer|InRange(Integer) GridX 0 (Variables|Default|GetMapWidth) true false) (Math|Integer|InRange(Integer) GridY 0 (Variables|Default|GetMapHeight) true false)) (+ (* GridY (Variables|Default|GetMapWidth)) GridX)))

(fn GetTilePos
  (params (GridX :type Integer) (GridY :type Integer))
  ;[1 1 1] TileMap X,Y좌표에 따른 World Position 좌표 구하고 맵 범위검사
  (bind _bvalid (CallFunction|GridPositiontoIndex GridX GridY))
  (return _bvalid (+ (Transformation|GetActorLocation) (Math|Vector|MakeVector (* GridX (Variables|Default|GetMapSizeX) 5.0) 2.0 (* GridY (Variables|Default|GetMapSizeY) -5.0)))))